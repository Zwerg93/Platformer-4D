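; BP_GrappleHook is a grapple hook projectile actor that flies out until it reaches a maximum range.
; On BeginPlay it passes its Velocity variable to the ProjectileMovement component and records its start location.
; Each Tick it measures the distance from that start point and destroys itself at MaxDistance.
; The event graph contains no hit, attach or pull logic.
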(event EventBeginPlay
  (Variables|/Script/Engine.MovementComponent|SetVelocity (Variables|Components|GetProjectileMovement) (Variables|Default|GetVelocity))
  (Variables|Default|SetStartLocation (Transformation|GetActorLocation)))

(event EventTick
  (params (DeltaSeconds :type Float%20%28single-precision%29))
  (if (>= (Math|Vector|Distance(Vector) (Variables|Default|GetStartLocation) (Transformation|GetActorLocation)) (Variables|Default|GetMaxDistance))
    (Actor|DestroyActor)))

(fn ConstructionScript)